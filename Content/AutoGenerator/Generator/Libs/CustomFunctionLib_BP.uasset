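; Blueprint function library for the auto generator that provides axis-aligned box overlap tests.
; BoxIntersect compares the min and max bounds of two boxes on X, Y and Z, reporting no overlap if any axis is separated and counting touching faces as intersecting.
; BoxIntersectWithArray runs that test for a query box against an array of boxes and returns whether any of them intersects it.
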(fn BoxIntersectwithArray
  (params (QueryBox :type Box%20Structure) (TestsBox :type Array%20of%20Box%20Structures))
  (bind _array_element (Utilities|Array|ForEachLoopwithBreak TestsBox :!label _label)
    (:LoopBody
      (bind _isintersect (CallFunction|BoxIntersect _array_element QueryBox))
      (if _isintersect
        (Utilities|FlowControl|Sequence
          (:then_0
            (goto _label Break))
          (:then_1
            (return true)))))
    (:Completed
      (return false))))

(fn BoxIntersect
  (params (BoxA :type Box%20Structure) (BoxB :type Box%20Structure))
  (bind (_min _max) (Utilities|Struct|BreakBox BoxA))
  (bind (_min_2 _max_2) (Utilities|Struct|BreakBox BoxB))
  (bind (_x _y _z) (Math|Vector|BreakVector _min))
  (bind (_x_2 _y_2 _z_2) (Math|Vector|BreakVector _min_2))
  (bind (_x_3 _y_3 _z_3) (Math|Vector|BreakVector _max_2))
  (bind (_x_4 _y_4 _z_4) (Math|Vector|BreakVector _max))
  (if (Math|Boolean|ORBoolean (> _x _x_3) (> _x_2 _x_4) (> _y _y_3) (> _y_2 _y_4) (> _z _z_3) (> _z_2 _z_4))
    (return false)
    (else
      (return true))))